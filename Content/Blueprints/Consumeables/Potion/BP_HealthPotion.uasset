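; Health potion pickup that applies an instant Gameplay Ability System effect to whatever overlaps it.
; Sphere overlap looks up the other actor's Ability System Component and, if valid, applies an InstantGameplayEffect spec at ActorLevel to it.
; The potion then removes itself through a short lifespan.
; An unconnected ApplyEffectToTarget branch remains in the graph and never runs.
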(event `self.Sphere.OnComponentBeginOverlap`
  (params (OverlappedComponent :type "PrimitiveComponent Object Reference") (OtherActor :type "Actor Object Reference") (OtherComp :type "PrimitiveComponent Object Reference") (OtherBodyIndex :type Integer) (bFromSweep :type Boolean) (SweepResult :type "HitResult Structure (by ref)"))
  (bind _returnvalue (`AbilitySystemBlueprintLibrary.GetAbilitySystemComponent` OtherActor))
  (`/Engine/EditorBlueprintResources/StandardMacros.IsValid` _returnvalue
    (:`Is Valid`
      (`AbilitySystemComponent.BP_ApplyGameplayEffectSpecToSelf` _returnvalue (`AbilitySystemComponent.MakeOutgoingSpec` _returnvalue (`self.InstantGameplayEffect`) (`self.ActorLevel`) (`AbilitySystemComponent.MakeEffectContext` _returnvalue)))
      (`self.SetLifeSpan` 0.2))))

(fn `UserConstructionScript`)